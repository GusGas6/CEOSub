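; Base interactable Blueprint for objects that a pawn repairs over time, tracked as a 0–100 State value.
; On the server, starting interaction runs a looping timer that raises State until it is full, then stops and clears the cached pawn.
; CanInteract allows one pawn at a time while repair is unfinished.
; Client start/stop events are placeholder prints for visuals, and Tick optionally draws color-coded State as debug text.
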(event `OnInteractionStarted_Client`
  ;[1 1 1] Use Those for visuals
  (`KismetSystemLibrary.PrintString` "*FIXING ANIM*"))

(event `Break_Debug`
  ;[1 0.5633 0] Debug button
  (set `self.State` 0.0))

(event `OnInteractionStopped_Client`
  ;[1 1 1] Use Those for visuals
  (`KismetSystemLibrary.PrintString` "*END FIXING ANIM*"))

(event `self.ReceiveTick`
  (params (DeltaSeconds :type "Float (single-precision)"))
  ;[1 1 1] Replace with UI progress bar. Leave it as a debug feature
  (if (not (`KismetSystemLibrary.IsDedicatedServer`))
    (if (`self.bDebugDrawState`)
      (`KismetSystemLibrary.DrawDebugString` (0.0 0.0 0.0) (`KismetStringLibrary.Conv_DoubleToString` (`self.State`)) self (`KismetMathLibrary.SelectColor` (`KismetMathLibrary.SelectColor` (struct :`R` 1.0 :`A` 1.0) (struct :`R` 1.0 :`G` 1.0 :`A` 1.0) (<= (`self.State`) 10.0)) (struct :`R` 0.038153 :`G` 1.0 :`A` 1.0) (<= (`self.State`) 75.0)) DeltaSeconds))))

(event `/Game/Blueprints/IBP_Interact.StartIneract`
  (params (InteractingPawn :type "Pawn Object Reference"))
  (set `self.Cached Interacting Pawn` InteractingPawn)
  (if (`KismetSystemLibrary.IsServer`)
    (bind _returnvalue (`KismetSystemLibrary.K2_SetTimerDelegate` (delegate `Repair`) (`self.RepairDelay`) true))
    (set `self.RepairTimerHandle` _returnvalue)
    (`self.OnInteractionStarted_Client`)
    (`KismetSystemLibrary.PrintString` (`KismetStringLibrary.Concat_StrStr` (`KismetSystemLibrary.GetDisplayName` self) "-Interaction: Start"))))

(event `Repair`
  (bind _output_get (set `self.State` (`KismetMathLibrary.FClamp` (+ (`self.State`) (`self.RepairSpeed`)) 0.0 100.0)))
  (if (>= _output_get 100.0)
    (`self.StopInteract` (`self.Cached Interacting Pawn`))))

(event `/Game/Blueprints/IBP_Interact.StopInteract`
  (params (InteractingPawn :type "Pawn Object Reference"))
  (if (`KismetSystemLibrary.IsServer`)
    (if (`KismetSystemLibrary.K2_IsValidTimerHandle` (`self.RepairTimerHandle`))
      (`KismetSystemLibrary.K2_ClearAndInvalidateTimerHandle` (`self.RepairTimerHandle`))
      (`self.OnInteractionStopped_Client`))
    (set `self.Cached Interacting Pawn` null) ; Clear Ref
    (`KismetSystemLibrary.PrintString` (`KismetStringLibrary.Concat_StrStr` (`KismetSystemLibrary.GetDisplayName` self) "-Interaction: Stop"))))

(fn `CanInteract`
  (returns (Output :type Boolean))
  (return (and (<= (`self.State`) 99.0) (not (`KismetSystemLibrary.IsValid` (`self.Cached Interacting Pawn`))))))

(fn `UserConstructionScript`)